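; TestingGrid is a test Blueprint that exercises AStarBetweenTiles, an A* query between two 2D tile coordinates, and prints the results.
; On BeginPlay it runs the query in both directions between two fixed tiles.
; Each Tick it queries from the stored Current tile to a random target built from a single integer, so X equals Y, then makes that target the new Current.
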(event EventBeginPlay
  (Variables|Default|SetCurrent "")
  (bind _returnvalue (Class|GridSystem|AStarBetweenTiles "(X=0.000000,Y=0.000000)" "(X=5.000000,Y=10.000000)"))
  (Development|PrintString (Utilities|String|ToString(Vector2d) _returnvalue) true true "(R=0.000000,G=0.660000,B=1.000000,A=1.000000)" 2e+01)
  (bind _returnvalue_2 (Class|GridSystem|AStarBetweenTiles "(X=5.000000,Y=10.000000)" "(X=0.000000,Y=0.000000)"))
  (Development|PrintString (Utilities|String|ToString(Vector2d) _returnvalue_2) true true "(R=0.000000,G=0.660000,B=1.000000,A=1.000000)" 2e+01))

(event EventTick
  (params (DeltaSeconds :type Float%20%28single-precision%29))
  (bind _output_get (Variables|Default|SetVector1 (Math|Conversions|ToVector2D(Vector) (Math|Conversions|ToVector(Float) (Math|Random|RandomIntegerinRange 0 49)))))
  (bind _returnvalue (Class|GridSystem|AStarBetweenTiles (Variables|Default|GetCurrent) _output_get))
  (Variables|Default|SetCurrent _output_get)
  (Development|PrintString (Utilities|String|ToString(Vector2d) _returnvalue) true true "(R=0.000000,G=0.660000,B=1.000000,A=1.000000)" 1.0))

(fn ConstructionScript)