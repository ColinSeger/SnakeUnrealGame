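; Snake body segment actor that ends play when a SnakePawn overlaps it.
; Its Sphere1 collision switches to query and physics two seconds after BeginPlay.
; On overlap with a SnakePawn, it shows the BP_NextMap widget, destroys every SnakePawn in the level and forces garbage collection.
; An unconnected branch that destroys only the cast pawn never runs.
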(event EventBeginPlay
  (Utilities|FlowControl|Delay 2.0)
  (Collision|SetCollisionEnabled (Variables|Default|GetSphere1) "QueryAndPhysics"))

(event EventTick
  (params (DeltaSeconds :type Float%20%28single-precision%29)))

(event Collision|EventActorBeginOverlap
  (params (OtherActor :type Actor%20Object%20Reference))
  (Utilities|Casting|CastToSnakePawn OtherActor)
  (bind _returnvalue (UserInterface|CreateWidget "/Game/UI/BP_NextMap.BP_NextMap_C" (Game|GetPlayerController 0)))
  (UserInterface|Viewport|AddtoViewport _returnvalue 0)
  (bind _outactors (Actor|GetAllActorsOfClass "/Script/SnakeUnreal.SnakePawn"))
  (Actor|DestroyActor _outactors)
  (Utilities|Platform|CollectGarbage))

(fn ConstructionScript)