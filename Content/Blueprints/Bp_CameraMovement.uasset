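; Camera pawn for what appears to be a two-player snake game, acting as the shared input hub.
; On BeginPlay it makes player controller 0 possess it, then, if its owner is valid, adds the Enhanced Input mapping and caches all SnakeTest3 actors.
; Two input actions steer the first and second cached snakes by array index.
; A camera action yaws the root and shifts the camera along its relative X to change distance.
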(event Input|EnhancedActionEvents|EnhancedInputActionPlayer2InputAction
  (params (ActionValue :type Vector%202D%20Structure) (ElapsedSeconds :type Float%20%28double-precision%29) (TriggeredSeconds :type Float%20%28double-precision%29) (InputAction :type Input%20Action%20Object%20Reference :default "/Game/Input/Player2InputAction.Player2InputAction"))
  (for (_array_element _array_index) (Variables|Default|GetSNakes)
    (if (== _array_index 1)
      (Default|ChangeDirection _array_element ActionValue))))

(event Input|EnhancedActionEvents|EnhancedInputActionInputCameraMovement
  (params (ActionValue :type Vector%202D%20Structure) (ElapsedSeconds :type Float%20%28double-precision%29) (TriggeredSeconds :type Float%20%28double-precision%29) (InputAction :type Input%20Action%20Object%20Reference :default "/Game/Input/InputCameraMovement.InputCameraMovement"))
  (bind _returnvalue (* ActionValue "(X=10.000000,Y=2.000000)"))
  (bind (_x _y) (Math|Vector2D|BreakVector2D _returnvalue))
  (CallFunction|ChangeCameraDistance _y)
  (CallFunction|RotateCamera _x))

(event Input|EnhancedActionEvents|EnhancedInputActionPlayerInputAction
  (params (ActionValue :type Vector%202D%20Structure) (ElapsedSeconds :type Float%20%28double-precision%29) (TriggeredSeconds :type Float%20%28double-precision%29) (InputAction :type Input%20Action%20Object%20Reference :default "/Game/Input/PlayerInputAction.PlayerInputAction"))
  (for (_array_element _array_index) (Variables|Default|GetSNakes)
    (if (== _array_index 0)
      (Default|ChangeDirection _array_element ActionValue))))

(event EventBeginPlay
  (Pawn|Possess (Game|GetPlayerController 0) self)
  (Utilities|IsValid (Components|GetOwner)
    (:Is%20Valid
      (Input|AddMappingContext (PlayerController|LocalPlayerSubsystems|GetEnhancedInputLocalPlayerSubsystem (Game|GetPlayerController 0)) "/Game/Input/PlayerKeyInputs.PlayerKeyInputs" 0 "(bIgnoreAllPressedKeysUntilRelease=True,bForceImmediately=False,bNotifyUserSettings=False)")
      (bind _outactors (Actor|GetAllActorsOfClass "/Game/Player/SnakeTest3.SnakeTest3_C"))
      (Variables|Default|SetSNakes _outactors))))

(fn ConstructionScript)

(fn RotateCamera
  (params (Speed :type Float%20%28double-precision%29))
  (Transformation|SetRelativeRotation (Variables|Default|GetDefaultSceneRoot) (Math|Rotator|CombineRotators (Transformation|GetWorldRotation (Variables|Default|GetDefaultSceneRoot)) (Math|Rotator|MakeRotator 0.0 0.0 Speed)) false false))

(fn ChangeCameraDistance
  (params (DirectionAndSpeed :type Float%20%28double-precision%29))
  (Transformation|SetRelativeLocation (Variables|Default|GetCamera) (+ (Variables|/Script/Engine.SceneComponent|GetRelativeLocation (Variables|Default|GetCamera)) (Math|Vector|MakeVector DirectionAndSpeed 0.0 0.0)) false false))